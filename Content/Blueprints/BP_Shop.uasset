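; BP_Shop is a damageable shop actor with a health component and a health bar widget.
; On damage it updates the bar's percent from current over max health.
; The first drop to or below the low-health threshold plays an audio cue once, guarded by an IsLow flag that is never reset here.
; The death event is bound but does nothing.
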(event `self.BP_HealthComponent.OnDied`)

(event `self.BP_HealthComponent.OnDamaged`
  (params (Damage :type "Float (double-precision)") (NewHealth :type "Float (double-precision)"))
  (`|ExecutionSequence`
    (:`then_0`
      (if (<= (/ NewHealth (`/Game/Components/BP_HealthComponent.MaxHealth` (`self.BP_HealthComponent`))) (`self.LowHealthPercent`))
        (if (not (`self.IsLow`))
          (set `self.IsLow` true)
          (`AudioComponent.Play` (`self.Audio`) 0.0))))
    (:`then_1`
      (bind _aswbp_health_bar (cast `/Game/UI/WBP_HealthBar` (`WidgetComponent.GetUserWidgetObject` (`self.HealthBar`))))
      (`ProgressBar.SetPercent` (`/Game/UI/WBP_HealthBar.HealthBar` _aswbp_health_bar) (/ NewHealth (`/Game/Components/BP_HealthComponent.MaxHealth` (`self.BP_HealthComponent`)))))))

(fn `UserConstructionScript`)