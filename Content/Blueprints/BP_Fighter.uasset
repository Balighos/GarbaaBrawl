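; BP_Fighter is a fighter character that reacts to damage and death events from its BP_HealthComponent, whether player-controlled or not.
; Damage plays a random hurt sound at its location and prints the new health.
; Death disables movement and capsule collision and turns the mesh into a physics ragdoll.
; For a player-controlled fighter, death also shows the WBP_GameOver widget after a short delay, with cursor and UI-only input.
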(event `self.BP_HealthComponent.OnDamaged`
  (params (Damage :type "Float (double-precision)") (NewHealth :type "Float (double-precision)"))
  (`GameplayStatics.PlaySoundAtLocation` (`KismetArrayLibrary.Array_Random` (`self.HurtSounds`)) (`self.K2_GetActorLocation` (`self.GetOwner`)) (struct) 1.0 1.0 0.0 null null null null)
  (`KismetSystemLibrary.PrintString` (`KismetStringLibrary.Conv_DoubleToString` NewHealth)))

(event `self.BP_HealthComponent.OnDied`
  (bind _returnvalue (`GameplayStatics.GetPlayerController` 0))
  (bind _mesh (`self.Mesh`))
  (`KismetSystemLibrary.PrintString` "DEAD")
  (`CharacterMovementComponent.DisableMovement` (`self.CharacterMovement`))
  (`PrimitiveComponent.SetCollisionProfileName` _mesh "Ragdoll" true)
  (`PrimitiveComponent.SetSimulatePhysics` _mesh true)
  (`PrimitiveComponent.SetCollisionEnabled` (`self.CapsuleComponent`) "NoCollision")
  (if (`Controller.IsPlayerController` (`self.GetController`))
    (`KismetSystemLibrary.Delay` 1.0)
    (bind _returnvalue_2 (`|CreateWidget` "/Game/UI/WBP_GameOver.WBP_GameOver_C" _returnvalue))
    (set `PlayerController.bShowMouseCursor` true _returnvalue)
    (`UserWidget.AddToViewport` _returnvalue_2 0)
    (`WidgetBlueprintLibrary.SetInputMode_UIOnlyEx` _returnvalue _returnvalue_2)))

(fn `UserConstructionScript`)