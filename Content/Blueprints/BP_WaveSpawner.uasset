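; Wave spawner actor that spawns growing groups of enemies around its own location.
; BeginPlay starts a wave immediately and sets a timer, with no looping specified, to call StartWave after TimeBetweenWaves.
; Each wave increments CurrentWave and spawns a base count plus a linear per-wave increase, using the class taken from EnemyClass.
; Spawns use random reachable navigation points within SpawnRadius, raised vertically and adjusted for collision but always spawned.
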(event `self.ReceiveBeginPlay`
  (`self.StartWave`)
  (`KismetSystemLibrary.K2_SetTimerDelegate` (delegate `StartWave`) (`self.TimeBetweenWaves`)))

(event `StartWave`
  (set `self.CurrentWave` (+ (`self.CurrentWave`) 1))
  (for _ (range 1 (+ (+ (* (- (`self.CurrentWave`) 1) (`self.WaveIncrease`)) (`self.EnemiesPerWave`)) 1))
    (`|SpawnActorFromClass` (`GameplayStatics.GetObjectClass` (`self.EnemyClass`)) (`KismetMathLibrary.Conv_VectorToTransform` (+ (`NavigationSystemV1.K2_GetRandomReachablePointInRadius` (`self.K2_GetActorLocation`) (`self.SpawnRadius`) null null) (`KismetMathLibrary.MakeVector` 0.0 0.0 100.0))) "AdjustIfPossibleButAlwaysSpawn" "MultiplyWithRoot" null null)))

(fn `UserConstructionScript`)