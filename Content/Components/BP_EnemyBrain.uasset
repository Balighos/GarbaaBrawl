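; Enemy AI component that makes its owning pawn attack the player or shops until it dies.
; A one-second looping timer prioritises a nearby player, otherwise targets a shop, falling back to the player if none is found.
; It closes in with AIMoveTo, then punches through BP_PunchComponent or damages the shop directly with a punch montage.
; FindNearestShop returns at the first shop under BestDist, so its result may not be the nearest.
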(event `self.ReceiveBeginPlay`
  (bind _returnvalue (`self.GetOwner`))
  (bind _aspawn (cast `Pawn` (`self.GetOwner`)))
  (set `self.OwnerPawn` _aspawn)
  (set `self.HealthComp` (`Actor.GetComponentByClass` _returnvalue "/Game/Components/BP_HealthComponent.BP_HealthComponent_C"))
  (set `self.Puncher` (`Actor.GetComponentByClass` _returnvalue "/Game/Components/BP_PunchComponent.BP_PunchComponent_C"))
  (`KismetSystemLibrary.K2_SetTimerDelegate` (delegate `Think`) 1.0 true))

(event `Think`
  (bind _returnvalue (`GameplayStatics.GetPlayerPawn` 0))
  (bind _ownerpawn (`self.OwnerPawn`))
  (if (`/Game/Components/BP_HealthComponent.IsDead` (`self.HealthComp`))
    _
    (elif (<= (`Actor.GetDistanceTo` (`self.OwnerPawn`) (`GameplayStatics.GetPlayerPawn` 0)) (`self.PlayerPriorityDistance`))
      (if (<= (`Actor.GetDistanceTo` _ownerpawn _returnvalue) (`self.AttackDistance`)) :!label _label
        (`Actor.K2_SetActorRotation` (`self.OwnerPawn`) (`KismetMathLibrary.MakeRotator` 0.0 0.0 (.yaw (`KismetMathLibrary.MakeRotFromX` (- (`Actor.K2_GetActorLocation` _returnvalue) (`Actor.K2_GetActorLocation` _ownerpawn))))) false)
        (`KismetSystemLibrary.PrintString` "PUNCH TRY")
        (`/Game/Components/BP_PunchComponent.Punch` (`self.Puncher`))
        (else
          (`|AIMoveTo` _ownerpawn (0.0 0.0 0.0) _returnvalue 80.0)))
      (else
        (bind _shop (`self.FindNearestShop`))
        (bind _output_get (set `self.TargetShop` _shop))
        (if (`KismetSystemLibrary.IsValid` _output_get)
          (if (<= (`Actor.GetDistanceTo` (`self.OwnerPawn`) (`self.TargetShop`)) (`self.ShopAttackDistance`))
            (bind _ascharacter (cast `Character` (`self.OwnerPawn`)))
            (if (not (`AnimInstance.Montage_IsPlaying` (`SkeletalMeshComponent.GetAnimInstance` (`Character.Mesh` _ascharacter)) "/Game/Animations/AM_Punch.AM_Punch"))
              (`Character.PlayAnimMontage` _ascharacter "/Game/Animations/AM_Punch.AM_Punch" 1.0 "None")
              (`GameplayStatics.ApplyDamage` (`self.TargetShop`) (`self.ShopDamage`) null (`self.OwnerPawn`))
              (`KismetSystemLibrary.PrintString` "SHOP HIT"))
            (else
              (`|AIMoveTo` (`self.OwnerPawn`) (0.0 0.0 0.0) (`self.TargetShop`) 150.0)))
          (else
            (goto _label)))))))

(fn `FindNearestShop`
  (returns (Shop :type "Actor Object Reference"))
  (locals (BestDist :type "Float (double-precision)" :default 9999999999.0) (Best :type "Actor Object Reference"))
  (bind _outactors (`GameplayStatics.GetAllActorsOfClass` "/Game/Blueprints/BP_Shop.BP_Shop_C"))
  (for _array_element _outactors
    (bind _returnvalue (`Actor.GetDistanceTo` (`self.OwnerPawn`) _array_element))
    (if (< _returnvalue (`local.BestDist`))
      (set `local.BestDist` _returnvalue)
      (set `local.Best` _array_element)
      (return (`local.Best`))))
  (return (`local.Best`)))