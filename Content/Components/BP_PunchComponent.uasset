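; Actor component that gives its owning Character a melee punch attack with a cooldown.
; Punch plays the next montage from a cycling list and a random sound, then runs a sphere overlap in front of the owner.
; Each overlapped pawn takes damage, and Characters not controlled by a player are launched forward and up as knockback.
; A timer calls ResetPunch to re-enable punching.
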(fn `GetNextPunchMontage`
  (returns (Montage :type "AnimMontage Object Reference"))
  (bind _punchmontages (`self.PunchMontages`))
  (set `self.PunchIndex` (mod (+ (`self.PunchIndex`) 1) (`KismetArrayLibrary.Array_Length` _punchmontages)))
  (return (`|GetArrayItem` _punchmontages (`self.PunchIndex`))))

(fn `Punch`
  (bind _returnvalue (`self.GetOwner`))
  (bind _returnvalue_2 (`self.GetOwner`))
  (`KismetSystemLibrary.PrintString` "CALLED")
  (if (`self.CanPunch`)
    (set `self.CanPunch` false)
    (`KismetSystemLibrary.K2_SetTimer` null "ResetPunch" (`self.Cooldown`))
    (bind _ascharacter (cast `Character` (`self.GetOwner`)))
    (bind _montage (`self.GetNextPunchMontage`))
    (`Character.PlayAnimMontage` _ascharacter _montage 1.0 "None")
    (`GameplayStatics.PlaySoundAtLocation` (`KismetArrayLibrary.Array_Random` (`self.PunchSounds`)) (`Actor.K2_GetActorLocation` (`self.GetOwner`)) (struct) 1.0 1.0 0.0 null null null null)
    (bind _outactors (`KismetSystemLibrary.SphereOverlapActors` (+ (`Actor.K2_GetActorLocation` _returnvalue) (* (`Actor.GetActorForwardVector` _returnvalue) (`self.Range`))) (`self.Radius`) (`|MakeArray` "ObjectTypeQuery3" :!type "EObjectTypeQuery Enum") null (`|MakeArray` _returnvalue_2)))
    (for _array_element _outactors
      (`GameplayStatics.ApplyDamage` _array_element (`self.Damage`) null _returnvalue_2)
      (bind _ascharacter_2 (cast `Character` _array_element))
      (if (not (`Pawn.IsPlayerControlled` _ascharacter_2))
        (`Character.LaunchCharacter` _ascharacter_2 (+ (* (`Actor.GetActorForwardVector` (`self.GetOwner`)) (`self.KnockbackForce`)) (`KismetMathLibrary.MakeVector` 0.0 0.0 (`self.KnockbackUp`))) true true)))))

(fn `ResetPunch`
  (set `self.CanPunch` true))