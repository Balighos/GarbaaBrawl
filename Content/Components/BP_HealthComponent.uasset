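; Health component that tracks an actor's health and death state.
; On BeginPlay it fills Health to MaxHealth and binds to the owner's OnTakeAnyDamage.
; Damage lowers clamped Health and broadcasts OnDamaged, then sets IsDead and broadcasts OnDied at zero.
; Heal restores clamped Health unless dead and prints the new value to screen.
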(event `OnTakeAnyDamage_Event`
  (params (DamagedActor :type "Actor Object Reference") (Damage :type "Float (single-precision)") (DamageType :type "DamageType Object Reference") (InstigatedBy :type "Controller Object Reference") (DamageCauser :type "Actor Object Reference"))
  (bind _health (`self.Health`))
  (if (not (`self.IsDead`))
    (set `self.Health` (`KismetMathLibrary.FClamp` (- (`self.Health`) Damage) 0.0 (`self.MaxHealth`)))
    (`self.OnDamaged` Damage _health)
    (if (<= _health 0.0)
      (set `self.IsDead` true)
      (`self.OnDied`))))

(event `self.ReceiveBeginPlay`
  (set `self.Health` (`self.MaxHealth`))
  (add `Actor.OnTakeAnyDamage` (`self.GetOwner`) (delegate `OnTakeAnyDamage_Event`)))

(fn `Heal`
  (params (Amount :type "Float (double-precision)"))
  (if (not (`self.IsDead`))
    (bind _output_get (set `self.Health` (`KismetMathLibrary.FClamp` (+ (`self.Health`) Amount) 0.0 (`self.MaxHealth`))))
    (`KismetSystemLibrary.PrintString` (`KismetStringLibrary.Conv_DoubleToString` _output_get))))